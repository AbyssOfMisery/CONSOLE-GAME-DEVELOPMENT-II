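; BP_PlayerPawn is a player pawn Blueprint that detects damage boost and invincibility pickups near the player.
; Every tick it box-traces for PhysicsBody objects between two offsets from player 0's location, with debug drawing left on.
; On a hit, it casts the actor to each pickup class and sets Touched on the matching one, leaving the effect outside this Blueprint.
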(event `self.ReceiveBeginPlay`)

(event `self.ReceiveTick`
  (params (DeltaSeconds :type "Float (single-precision)"))
  (bind _returnvalue (`self.K2_GetActorLocation` (`GameplayStatics.GetPlayerPawn` 0)))
  (bind (_outhit _returnvalue_2) (`KismetSystemLibrary.BoxTraceSingleForObjects` :`Start` (+ _returnvalue (`self.start`)) :`End` (+ (`self.end`) _returnvalue) :`HalfSize` (20.0 20.0 40.0) :`ObjectTypes` (`|MakeArray` "ObjectTypeQuery4" :!type "EObjectTypeQuery Enum") :`bTraceComplex` true :`DrawDebugType` "ForDuration"))
  (if _returnvalue_2
    (`|ExecutionSequence`
      (:`then_0`
        (bind (_bblockinghit _binitialoverlap _time _distance _location _impactpoint _normal _impactnormal _physmat _hitactor) (`GameplayStatics.BreakHitResult` _outhit))
        (bind _asmy_damage_boost_pickup (cast `/Game/BluePrints/MyDamage_Boost_Pickup` _hitactor))
        (set `/Game/BluePrints/MyDamage_Boost_Pickup.touched` true _asmy_damage_boost_pickup))
      (:`then_1`
        (bind _asmy_invincibility_pickup (cast `/Game/BluePrints/MyInvincibility_Pickup` _hitactor))
        (set `/Game/BluePrints/MyInvincibility_Pickup.touched` true _asmy_invincibility_pickup)))))

(fn `UserConstructionScript`)