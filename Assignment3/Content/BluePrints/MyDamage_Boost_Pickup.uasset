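; Damage boost pickup that temporarily raises the damage of the player's current weapon.
; Pressing F while the Touched flag is set casts the owner to BP_PlayerPawn and quadruples the current weapon's BaseDamage for ten seconds.
; A timer then sets the current weapon's BaseDamage to a hardcoded value instead of restoring the original.
; Nothing in these graphs sets Touched, and the overlap event is disabled.
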(event `Key|F`
  (params (Key :type "Key Structure"))
  (:`Pressed`
    (if (`self.touched`)
      (bind _asbp_player_pawn (cast `/Game/BluePrints/BP_PlayerPawn` (`self.GetOwner`)))
      (bind _currentweapon (`TPSCharacter.CurrentWeapon` _asbp_player_pawn))
      (set `TPSWeapon.BaseDamage` (* (`TPSWeapon.BaseDamage` _currentweapon) 4.0) _currentweapon)
      (`KismetSystemLibrary.K2_SetTimerDelegate` (delegate `reset`) 10.0))))

(event `reset`
  (set `TPSWeapon.BaseDamage` 20.0 (`TPSCharacter.CurrentWeapon` (stale `Key|F` _asbp_player_pawn))))

(fn `UserConstructionScript`)