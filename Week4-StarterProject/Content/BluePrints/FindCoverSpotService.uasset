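; AI behavior tree service that finds a cover spot hidden from the player and writes it to the FoundCoverSpot blackboard key.
; Each tick, it sphere-overlaps for BP_CoverTemp actors in range and evaluates only the nearest.
; If a raised trace from that cover to the player is unobstructed, it checks child CoverSpotV2s in their first state or used by this pawn.
; It picks the first spot whose trace to the player hits that cover.
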(event `self.ReceiveTickAI`
  (params (OwnerController :type "AIController Object Reference") (ControlledPawn :type "Pawn Object Reference") (DeltaSeconds :type "Float (single-precision)"))
  (bind (_foundcover _coverspot) (`self.FindCoverSpotOverlap` ControlledPawn))
  (if _foundcover
    (`BTFunctionLibrary.SetBlackboardValueAsObject` (`self.FoundCoverSpot`) _coverspot)))

(fn `FindCoverSpotOverlap`
  (params (Owner :type "Pawn Object Reference"))
  (returns (foundCover :type Boolean) (CoverSpot :type "/Game/BluePrints/CoverSpotV2 Object Reference"))
  (bind _returnvalue (`GameplayStatics.GetPlayerPawn` 0))
  (bind _returnvalue_2 (`GameplayStatics.GetPlayerPawn` 0))
  (bind _outactors (`KismetSystemLibrary.SphereOverlapActors` (`Actor.K2_GetActorLocation` Owner) (`self.Range`) (`|MakeArray` "ObjectTypeQuery2" :!type "EObjectTypeQuery Enum") "/Game/BluePrints/BP_CoverTemp.BP_CoverTemp_C"))
  (bind _sorted_array (`DistanceSort.Distance_Sort` _outactors Owner))
  (bind (_output_distance _output_actor) (break `Actor_Dist` (`|GetArrayItem` _sorted_array)))
  (for _array_element (`|MakeArray` _output_actor)
    (bind _asbp_cover_temp (cast `/Game/BluePrints/BP_CoverTemp` _array_element)
      (:`then`
        (if (`KismetSystemLibrary.IsValid` _returnvalue_2)
          (bind (_outhit _returnvalue_3) (`KismetSystemLibrary.LineTraceSingle` (+ (`Actor.K2_GetActorLocation` _asbp_cover_temp) (0.0 0.0 200.0)) (`Actor.K2_GetActorLocation` _returnvalue_2) "TraceTypeQuery1" false (`|MakeArray` _returnvalue_2 :!type "Actor Object Reference")))
          (if (not _returnvalue_3)
            (for _array_element_2 (`/Game/BluePrints/BP_CoverTemp.CoverSpots` _asbp_cover_temp)
              (bind _ascover_spot_v2 (cast `/Game/BluePrints/CoverSpotV2` (`ChildActorComponent.ChildActor` _array_element_2)))
              (if (or (`|EnumEquality` (`/Game/BluePrints/CoverSpotV2.CurrentState` _ascover_spot_v2) "NewEnumerator0") (== (`/Game/BluePrints/CoverSpotV2.CurrentUser` _ascover_spot_v2) (`self.ControlledPawn`)))
                (if (`KismetSystemLibrary.IsValid` _returnvalue)
                  (bind (_outhit_2 _returnvalue_4) (`KismetSystemLibrary.LineTraceSingle` (`Actor.K2_GetActorLocation` _ascover_spot_v2) (`Actor.K2_GetActorLocation` _returnvalue) "TraceTypeQuery4"))
                  (if _returnvalue_4
                    (if (== (`.HitActor` (`GameplayStatics.BreakHitResult` _outhit_2)) _asbp_cover_temp)
                      (return true _ascover_spot_v2)))))))))
      (:`CastFailed`
        (return false null))))
  (return false null))